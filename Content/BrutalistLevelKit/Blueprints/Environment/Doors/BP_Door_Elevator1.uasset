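; BP_Door_Elevator1 is a two-panel sliding elevator door that opens and closes through an Activate event, unless IsLocked or HingeMode is set.
; Activate toggles Open, plays a sound and runs one timeline forward or in reverse to slide both panels along relative X.
; The Open flag reads inverted: it is false after forward play, when the finished timeline waits three seconds and calls Activate again to auto-close.
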(event Collision|EventActorBeginOverlap
  (params (OtherActor :type Actor%20Object%20Reference))
  (|CallParentFunction OtherActor) ; This node is disabled and will not be called.\nDrag off pins to build functionality.
)

(event EventTick
  (params (DeltaSeconds :type Float%20%28single-precision%29))
  (|CallParentFunction DeltaSeconds) ; This node is disabled and will not be called.\nDrag off pins to build functionality.
)

(event EventActivate
  (bind _returnvalue (Transformation|GetActorLocation))
  (bind _door2 (Variables|Default|GetDoor2))
  (bind _door (Variables|Default|GetDoor))
  (bind _relativelocation (Variables|/Script/Engine.SceneComponent|GetRelativeLocation _door))
  (bind _relativelocation_2 (Variables|/Script/Engine.SceneComponent|GetRelativeLocation _door2))
  (if (not (or (Variables|Default|GetIsLocked) (Variables|Default|GetHingeMode)))
    ;[1 1 1] Level Object Activation
    (if (Variables|Default|GetOpen)
      (Variables|Default|SetOpen false)
      (Audio|PlaySoundatLocation "/Game/EMsAssets/Audio/SoundSnap/SoundEffects/Doors/123159-Elevator_door_open_from_inside_the_elevator_with_a_clunk.123159-Elevator_door_open_from_inside_the_elevator_with_a_clunk" _returnvalue "0, 0, 0" 1.0 1.0 0.0 "/Game/EMsAssets/Audio/BasicSoundAttenuation.BasicSoundAttenuation" 0 0 0)
      (bind (_direction _door1opening _door2opening) (Timeline|Timeline_0 Play)
        (:Update
          ;[1 1 1] Door 1
          (Transformation|SetRelativeLocation _door (Math|Vector|MakeVector (+ _door2opening 1.561617) (.y _relativelocation) (.z _relativelocation)) false false)
          ;[1 1 1] Door 2
          (Transformation|SetRelativeLocation _door2 (Math|Vector|MakeVector (+ _door1opening 49.288483) (.y _relativelocation_2) (.z _relativelocation_2)) false false))
        (:Finished
          (if (not (Variables|Default|GetOpen))
            (Utilities|FlowControl|Delay 3.0)
            (if (not (Variables|Default|GetOpen))
              (CallFunction|Activate)))))
      (else
        (Variables|Default|SetOpen true)
        (Audio|PlaySoundatLocation "/Game/EMsAssets/Audio/SoundSnap/SoundEffects/Doors/123142-Elevator_door_close_from_inside_the_elevator_2.123142-Elevator_door_close_from_inside_the_elevator_2" _returnvalue "0, 0, 0" 1.0 1.0 0.0 "/Game/EMsAssets/Audio/BasicSoundAttenuation.BasicSoundAttenuation" 0 0 0)
        (Timeline|Timeline_0 Reverse)))))

(fn ConstructionScript
  (|CallParentFunction))