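; Basic swinging door from the Brutalist Level Kit that toggles open and closed on Activate, unless it is locked or in hinge mode.
; A timeline drives the door's yaw relative to its starting rotation, playing forward or in reverse with a sound at each toggle.
; After the forward swing finishes, it waits three seconds and re-activates itself to swing back.
; The Open flag reads inverted: it is false during the forward swing.
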(event EventBeginPlay
  (|CallParentFunction)
  (Variables|Default|SetRelativeYaw (.yaw (Variables|/Script/Engine.SceneComponent|GetRelativeRotation (Variables|Default|GetDoor)))))

(event Collision|EventActorBeginOverlap
  (params (OtherActor :type Actor%20Object%20Reference))
  (|CallParentFunction OtherActor) ; This node is disabled and will not be called.\nDrag off pins to build functionality.
)

(event EventTick
  (params (DeltaSeconds :type Float%20%28single-precision%29))
  (|CallParentFunction DeltaSeconds) ; This node is disabled and will not be called.\nDrag off pins to build functionality.
)

(event EventActivate
  (bind _returnvalue (Transformation|GetActorLocation))
  (bind _door (Variables|Default|GetDoor))
  (bind _relativerotation (Variables|/Script/Engine.SceneComponent|GetRelativeRotation _door))
  (if (not (or (Variables|Default|GetIsLocked) (Variables|Default|GetHingeMode)))
    ;[1 1 1] Level Object Activation
    (if (Variables|Default|GetOpen)
      (Variables|Default|SetOpen false)
      (Audio|PlaySoundatLocation "/Game/EMsAssets/Audio/SoundSnap/SoundEffects/Doors/240947-door_office_open-02.240947-door_office_open-02" _returnvalue "0, 0, 0" 0.8 1.0 0.0 "/Game/EMsAssets/Audio/BasicSoundAttenuation.BasicSoundAttenuation" 0 0 0)
      (bind _dooropening (Timeline|Timeline_0 Play)
        (:Update
          (Transformation|SetRelativeRotation _door (Math|Rotator|MakeRotator (.roll _relativerotation) (.pitch _relativerotation) (+ _dooropening (Variables|Default|GetRelativeYaw))) false false))
        (:Finished
          (if (not (Variables|Default|GetOpen))
            (Utilities|FlowControl|Delay 3.0)
            (if (not (Variables|Default|GetOpen))
              (CallFunction|Activate)))))
      (else
        (Variables|Default|SetOpen true)
        (Audio|PlaySoundatLocation "/Game/EMsAssets/Audio/SoundSnap/SoundEffects/Doors/240947-door_office_close-02.240947-door_office_close-02" _returnvalue "0, 0, 0" 0.8 1.0 0.0 "/Game/EMsAssets/Audio/BasicSoundAttenuation.BasicSoundAttenuation" 0 0 0)
        (Timeline|Timeline_0 Reverse)))))

(fn ConstructionScript
  (|CallParentFunction))