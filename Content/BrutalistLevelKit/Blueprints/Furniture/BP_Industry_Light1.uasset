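; BP_Industry_Light1 is an industrial light fixture that pairs a mesh with an emissive material and a point light.
; The construction script creates a dynamic material instance, applies the light color, and sets on/off from Active or, when Random is set, a seeded 50% roll.
; EnableLight and DisableLight switch the emissive color and point light visibility together.
; StartOff calls DisableLight on BeginPlay, overriding the constructed state.
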(event Custom|DisableLight
  (Rendering|Material|SetVectorParameterValue (Variables|Control|GetLightMatInst) "EmissiveColor" "(R=0.000000,G=0.000000,B=0.000000,A=1.000000)" :!class /Script/Engine.MaterialInstanceDynamic)
  (Rendering|SetVisibility (Variables|Default|GetPointLight1) false false))

(event Custom|EnableLight
  (Rendering|Material|SetVectorParameterValue (Variables|Control|GetLightMatInst) "EmissiveColor" (Variables|Default|GetColor) :!class /Script/Engine.MaterialInstanceDynamic)
  (Rendering|SetVisibility (Variables|Default|GetPointLight1) true false))

(event EventBeginPlay
  (|CallParentFunction)
  (if (Variables|Default|GetStartOff)
    (CallFunction|DisableLight)))

(event Collision|EventActorBeginOverlap
  (params (OtherActor :type Actor%20Object%20Reference))
  (|CallParentFunction OtherActor) ; This node is disabled and will not be called.\nDrag off pins to build functionality.
)

(event EventTick
  (params (DeltaSeconds :type Float%20%28single-precision%29))
  (|CallParentFunction DeltaSeconds) ; This node is disabled and will not be called.\nDrag off pins to build functionality.
)

(fn ConstructionScript
  (bind _furnituremesh (Variables|Default|GetFurnitureMesh))
  (bind _color (Variables|Default|GetColor))
  (bind _pointlight1 (Variables|Default|GetPointLight1))
  (|CallParentFunction)
  (LocalVariables|SetLocalRandom (select (Variables|Control|GetRandom) (Class|KismetMathLibrary|RandomBoolwithWeightfromStream 0.5 (Variables|Default|GetRandomSeedStruct)) (Variables|Default|GetActive)))
  (bind _returnvalue (Rendering|Material|CreateDynamicMaterialInstance _furnituremesh 0 (Rendering|Material|GetMaterial _furnituremesh 0) "None" :!class /Script/Engine.PrimitiveComponent))
  (bind _output_get (Variables|Control|SetLightMatInst _returnvalue))
  (Rendering|Material|SetVectorParameterValue _output_get "EmissiveColor" (select (LocalVariables|GetLocalRandom) _color "") :!class /Script/Engine.MaterialInstanceDynamic)
  (Rendering|SetVisibility _pointlight1 (LocalVariables|GetLocalRandom) false)
  (Rendering|Components|Light|SetLightColor _pointlight1 _color true))