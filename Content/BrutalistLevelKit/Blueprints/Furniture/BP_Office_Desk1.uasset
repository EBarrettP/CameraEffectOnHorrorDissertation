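; Procedural office desk prop from the Brutalist level kit that randomizes its desk, desktop items, chair and lamp.
; The construction script uses a seeded random stream to pick a desk mesh, then scatters items into HISMs at its "Desk"-prefixed sockets.
; Weighted rolls choose the chair and lamp meshes or a Cube stand-in, and the chair gets a random yaw.
; Activate toggles the Active flag when the lamp has a valid mesh.
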(event EventBeginPlay
  (|CallParentFunction) ; This node is disabled and will not be called.\nDrag off pins to build functionality.
)

(event Collision|EventActorBeginOverlap
  (params (OtherActor :type Actor%20Object%20Reference))
  (|CallParentFunction OtherActor) ; This node is disabled and will not be called.\nDrag off pins to build functionality.
)

(event EventTick
  (params (DeltaSeconds :type Float%20%28single-precision%29))
  (|CallParentFunction DeltaSeconds) ; This node is disabled and will not be called.\nDrag off pins to build functionality.
)

(event EventActivate
  (Utilities|IsValid (Variables|/Script/Engine.StaticMeshComponent|GetStaticMesh (Variables|Default|GetLamp))
    (:Is%20Valid
      (if (Variables|Default|GetActive)
        (Variables|Default|SetActive false)
        (else
          (Variables|Default|SetActive true))))))

(fn ConstructionScript
  (bind _chair (Variables|Default|GetChair))
  (bind _lamp (Variables|Default|GetLamp))
  (bind _deskmeshes (Variables|Default|GetDeskMeshes))
  (|CallParentFunction)
  ;[1 1 1] Handle Desk
  (Components|StaticMesh|SetStaticMesh (Variables|Default|GetFurnitureMesh) (Utilities|Array|Get(acopy) _deskmeshes (Math|Random|RandomIntegerinRangefromStream 0 (- (Utilities|Array|Length _deskmeshes) 1) (Variables|Default|GetRandomSeedStruct))))
  ;[1 1 1] Spawn Desk Items
  (CallFunction|SpawnMeshesfromSockets (Variables|Default|GetDeskItemHISMs) (Variables|Default|GetDeskItemMeshes) (Variables|Default|GetFurnitureMesh) "Desk")
  ;[1 1 1] Handle Chair
  (bind _returnvalue (Components|StaticMesh|SetStaticMesh _chair (select (Class|KismetMathLibrary|RandomBoolwithWeightfromStream 0.8 (Variables|Default|GetRandomSeedStruct)) "/Game/BrutalistLevelKit/Models/Props/Furnitures/SM_Office_Chair.SM_Office_Chair" "/Engine/BasicShapes/Cube.Cube")))
  (Rendering|SetVisibility _chair (not _returnvalue) false)
  (Transformation|SetRelativeScale3D _chair (Math|Vector|MakeVector (select (not _returnvalue) 1.0 0.05) (select (not _returnvalue) 1.0 0.05) (select (not _returnvalue) 1.0 0.05)))
  (Transformation|SetRelativeRotation _chair (Math|Rotator|MakeRotator 0.0 0.0 (+ (Math|Random|RandomFloatinRangefromStream -3e+01 3e+01 (Variables|Default|GetRandomSeedStruct)) 1.8e+02)) false false)
  ;[1 1 1] Handle Lamp
  (bind _returnvalue_2 (Components|StaticMesh|SetStaticMesh _lamp (select (Class|KismetMathLibrary|RandomBoolwithWeightfromStream 0.8 (Variables|Default|GetRandomSeedStruct)) "/Game/BrutalistLevelKit/Models/Props/Furnitures/Lights/SM_Desk_Lamp1.SM_Desk_Lamp1" "/Engine/BasicShapes/Cube.Cube")))
  (Rendering|SetVisibility _lamp (not _returnvalue_2) false)
  (Transformation|SetRelativeScale3D _lamp (Math|Vector|MakeVector (select (not _returnvalue_2) 1.0 0.05) (select (not _returnvalue_2) 1.0 0.05) (select (not _returnvalue_2) 1.0 0.05))))