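; BP_Keys is a keys pickup that changes doors when activated and plays a one-time sound when the player comes near.
; Activate calls ChangeDoors on its DoorChanger reference, fires PickUpKeys, then destroys the actor.
; Separately, a Player-tagged actor overlapping SoundBox plays a drop/crash sound at the FurnitureMesh location, and SoundBox destroys itself so it cannot repeat.
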(event OnComponentBeginOverlap(SoundBox)
  (params (OverlappedComponent :type Primitive%20Component%20Object%20Reference) (OtherActor :type Actor%20Object%20Reference) (OtherComp :type Primitive%20Component%20Object%20Reference) (OtherBodyIndex :type Integer) (bFromSweep :type Boolean) (SweepResult :type Hit%20Result%20Structure%20%28by%20ref%29))
  (if (Actor|ActorHasTag OtherActor "Player")
    (Audio|PlaySoundatLocation "/Game/EMsAssets/Audio/SoundSnap/SpookySounds/VendingMachine/86791-Crash_car_hood_object_drop-BLASTWAVEFX-21528.86791-Crash_car_hood_object_drop-BLASTWAVEFX-21528" (Transformation|GetWorldLocation (Variables|Default|GetFurnitureMesh)) "0, 0, 0" 0.7 1.0 0.0 "/Game/EMsAssets/Audio/BasicSoundAttenuation.BasicSoundAttenuation" 0 0 0)
    (Components|DestroyComponent (Variables|Default|GetSoundBox))))

(event EventBeginPlay)

(event Collision|EventActorBeginOverlap
  (params (OtherActor :type Actor%20Object%20Reference))
  (|CallParentFunction OtherActor) ; This node is disabled and will not be called.\nDrag off pins to build functionality.
)

(event EventTick
  (params (DeltaSeconds :type Float%20%28single-precision%29))
  (|CallParentFunction DeltaSeconds) ; This node is disabled and will not be called.\nDrag off pins to build functionality.
)

(event EventActivate
  (Default|ChangeDoors (Variables|Default|GetDoorChanger))
  (Default|CallPickUpKeys)
  (Actor|DestroyActor))

(fn ConstructionScript
  (|CallParentFunction))