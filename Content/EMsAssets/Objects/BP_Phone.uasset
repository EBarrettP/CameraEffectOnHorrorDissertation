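; BP_Phone is an interactive phone that vibrates continuously from BeginPlay until it is activated and destroyed.
; A self-restarting timeline drives the mesh's yaw wobble, the audio volume and the screen's glow together.
; The construction script creates the screen's dynamic material instance with the glow initially off.
; Activate tells DoorChanger to change doors and calls PickUpPhone before destroying the actor.
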(event Custom|Vibrate
  (bind _furnituremesh (Variables|Default|GetFurnitureMesh))
  (bind _relativerotation (Variables|/Script/Engine.SceneComponent|GetRelativeRotation _furnituremesh))
  (bind (_direction _newtrack_0 _newtrack_1) (Timeline|Timeline_0 PlayFromStart)
    (:Update
      (Transformation|SetRelativeRotation _furnituremesh (Math|Rotator|MakeRotator (.roll _relativerotation) (.pitch _relativerotation) _newtrack_0) false false)
      (Audio|Components|Audio|SetVolumeMultiplier (Variables|Default|GetAudio) (/ _newtrack_1 1e+01) :!class /Script/Engine.AudioComponent)
      (Rendering|Material|SetScalarParameterValue (Variables|Default|GetScreenMat) "Glowing" _newtrack_1 :!class /Script/Engine.MaterialInstanceDynamic))
    (:Finished
      (CallFunction|Vibrate))))

(event EventBeginPlay
  (CallFunction|Vibrate))

(event Collision|EventActorBeginOverlap
  (params (OtherActor :type Actor%20Object%20Reference))
  (|CallParentFunction OtherActor) ; This node is disabled and will not be called.\nDrag off pins to build functionality.
)

(event EventTick
  (params (DeltaSeconds :type Float%20%28single-precision%29))
  (|CallParentFunction DeltaSeconds) ; This node is disabled and will not be called.\nDrag off pins to build functionality.
)

(event EventActivate
  (Default|ChangeDoors (Variables|Default|GetDoorChanger))
  (Default|CallPickUpPhone)
  (Actor|DestroyActor))

(fn ConstructionScript
  (|CallParentFunction)
  (bind _returnvalue (Rendering|Material|CreateDynamicMaterialInstance "/Game/EMsAssets/GlowingMaterial.GlowingMaterial" "None" "None" :!class /Script/Engine.KismetMaterialLibrary))
  (bind _output_get (Variables|Default|SetScreenMat _returnvalue))
  (Rendering|Material|SetMaterial (Variables|Default|GetPhoneScreen) 0 _output_get)
  (Rendering|Material|SetScalarParameterValue _output_get "Glowing" 0.0 :!class /Script/Engine.MaterialInstanceDynamic))