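; Scare door that starts ajar and slams shut, taking a peeking SpookyMan figure with it, when the player enters its trigger box.
; The player-tagged overlap calls a one-shot SlamDoor, turns off SwitchTrigger's breathing and destroys the box.
; SlamDoor plays a sound and peek animation while a timeline rotates the door and incrementally shifts and turns SpookyMan, destroying him when finished.
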(event OnComponentBeginOverlap(SlamBox)
  (params (OverlappedComponent :type Primitive%20Component%20Object%20Reference) (OtherActor :type Actor%20Object%20Reference) (OtherComp :type Primitive%20Component%20Object%20Reference) (OtherBodyIndex :type Integer) (bFromSweep :type Boolean) (SweepResult :type Hit%20Result%20Structure%20%28by%20ref%29))
  (if (Actor|ActorHasTag OtherActor "Player")
    (CallFunction|SlamDoor)
    (Variables|/Game/EMsAssets/FCameraSwitchTrig.FCameraSwitchTrig_C|SetBreathing? (Variables|Default|GetSwitchTrigger) false)
    (Components|DestroyComponent (Variables|Default|GetSlamBox))))

(event Custom|SlamDoor
  (bind _door (Variables|Default|GetDoor))
  (bind _spookyman (Variables|Default|GetSpookyMan))
  (bind _spookyman_2 (Variables|Default|GetSpookyMan))
  (bind _returnvalue (Transformation|GetActorLocation _spookyman))
  (bind _returnvalue_2 (Transformation|GetActorRotation _spookyman_2))
  (bind _relativerotation (Variables|/Script/Engine.SceneComponent|GetRelativeRotation _door))
  (if (not (Variables|Default|GetDoorSlammed))
    (Variables|Default|SetDoorSlammed true)
    (Audio|PlaySoundatLocation "/Game/EMsAssets/Audio/SoundSnap/SpookySounds/155752-HUTCH-HD-SFX-2014-0014.155752-HUTCH-HD-SFX-2014-0014" (Transformation|GetWorldLocation (Variables|Default|GetDoor)) "0, 0, 0" 0.3 0.7 0.0 "/Game/EMsAssets/Audio/BasicSoundAttenuation.BasicSoundAttenuation" 0 0 0)
    (Components|Animation|PlayAnimation (Variables|/Game/EMsAssets/SpookySpecial/SpookyMan.SpookyMan_C|GetSkeletalMesh (Variables|Default|GetSpookyMan)) "/Game/TryingAnim/Eric/EricPeekingArm.EricPeekingArm" false)
    ;[0.2344 0.2344 0.2344] Rotate door and man to simulate closing the door
    (bind _newtrack_0 (Timeline|Timeline_1 PlayFromStart)
      (:Update
        (Transformation|SetRelativeRotation _door (Math|Rotator|MakeRotator (.roll _relativerotation) (.pitch _relativerotation) (+ _newtrack_0 (Variables|Default|GetRelativeYaw))) false false)
        (Transformation|SetActorLocation _spookyman (Math|Vector|MakeVector (.x _returnvalue) (- (.y _returnvalue) 1.3) (.z _returnvalue)) false false)
        (Transformation|SetActorRotation _spookyman_2 (Math|Rotator|MakeRotator (.roll _returnvalue_2) (.pitch _returnvalue_2) (+ (.yaw _returnvalue_2) 1.8))))
      (:Finished
        (Actor|DestroyActor (Variables|Default|GetSpookyMan))))))

(event EventBeginPlay
  (bind _door (Variables|Default|GetDoor))
  (bind _relativerotation (Variables|/Script/Engine.SceneComponent|GetRelativeRotation _door))
  (|CallParentFunction)
  (Transformation|SetRelativeRotation (Variables|Default|GetDoor) (Math|Rotator|MakeRotator (.roll _relativerotation) (.pitch _relativerotation) 25.0) false false))

(event Collision|EventActorBeginOverlap
  (params (OtherActor :type Actor%20Object%20Reference))
  (|CallParentFunction OtherActor) ; This node is disabled and will not be called.\nDrag off pins to build functionality.
)

(event EventTick
  (params (DeltaSeconds :type Float%20%28single-precision%29))
  (|CallParentFunction DeltaSeconds) ; This node is disabled and will not be called.\nDrag off pins to build functionality.
)

(fn ConstructionScript
  (|CallParentFunction))