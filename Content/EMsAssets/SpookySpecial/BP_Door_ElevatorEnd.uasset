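; BP_Door_ElevatorEnd is an elevator door that triggers the game's ending when activated.
; If unlocked, not in hinge mode and Open is set, it clears Open, disables player input, hides UI and slides both panels via a timeline.
; It then stops ambience, cuts to a faded screen with a laugh, waits, and either quits on a second run or loads ThirdPersonMap.
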(event EventBeginPlay
  (bind _returnvalue (Actor|GetActorOfClass "/Game/ThirdPerson/Blueprints/BP_ThirdPersonCharacter.BP_ThirdPersonCharacter_C"))
  (Variables|Default|SetThirdPerson _returnvalue)
  (bind _returnvalue_2 (Actor|GetActorOfClass "/Game/EMsAssets/Managers/AmbienceManager.AmbienceManager_C"))
  (Variables|Default|SetAmbience _returnvalue_2))

(event Collision|EventActorBeginOverlap
  (params (OtherActor :type Actor%20Object%20Reference))
  (|CallParentFunction OtherActor) ; This node is disabled and will not be called.\nDrag off pins to build functionality.
)

(event EventTick
  (params (DeltaSeconds :type Float%20%28single-precision%29))
  (|CallParentFunction DeltaSeconds) ; This node is disabled and will not be called.\nDrag off pins to build functionality.
)

(event EventActivate
  (bind _door2 (Variables|Default|GetDoor2))
  (bind _door (Variables|Default|GetDoor))
  (bind _thirdperson (Variables|Default|GetThirdPerson))
  (bind _relativelocation (Variables|/Script/Engine.SceneComponent|GetRelativeLocation _door))
  (bind _relativelocation_2 (Variables|/Script/Engine.SceneComponent|GetRelativeLocation _door2))
  (if (not (or (Variables|Default|GetIsLocked) (Variables|Default|GetHingeMode)))
    ;[1 1 1] Level Object Activation
    (if (Variables|Default|GetOpen)
      (Variables|Default|SetOpen false)
      (Audio|PlaySoundatLocation "/Game/EMsAssets/Audio/SoundSnap/SoundEffects/Doors/123159-Elevator_door_open_from_inside_the_elevator_with_a_clunk.123159-Elevator_door_open_from_inside_the_elevator_with_a_clunk" "0, 0, 0" "0, 0, 0" 1.0 1.0 0.0 "/Game/EMsAssets/Audio/BasicSoundAttenuation.BasicSoundAttenuation" 0 0 0)
      (Input|DisableInput _thirdperson (Pawn|GetLocalViewingPlayerController _thirdperson))
      (Default|HideUI _thirdperson)
      (bind (_direction _door1opening _door2opening) (Timeline|Timeline_0 PlayFromStart)
        (:Update
          ;[1 1 1] Door 1
          (Transformation|SetRelativeLocation _door (Math|Vector|MakeVector (+ _door2opening 1.561617) (.y _relativelocation) (.z _relativelocation)) false false)
          ;[1 1 1] Door 2
          (Transformation|SetRelativeLocation _door2 (Math|Vector|MakeVector (+ _door1opening 49.288483) (.y _relativelocation_2) (.z _relativelocation_2)) false false))
        (:Finished
          (Default|StopAmb (Variables|Default|GetAmbience))
          (CameraFades|StartCameraFade :self (Game|GetPlayerCameraManager 0) :ToAlpha 1.0 :Duration 0.1 :bHoldWhenFinished true)
          (Audio|PlaySound2D "/Game/EMsAssets/Audio/Laughter/WuhahahaHA.WuhahahaHA" 1.0 1.0 0.0 0 0)
          (Utilities|FlowControl|Delay 4.0)
          (bind _asmy_game_instance (Utilities|Casting|CastToMyGameInstance (Game|GetGameInstance)))
          (if (Variables|/Game/EMsAssets/MyGameInstance.MyGameInstance_C|GetSecondRun _asmy_game_instance)
            (Game|QuitGame 0 "Quit" false)
            (else
              (Game|OpenLevel(byObjectReference) "/Game/ThirdPerson/Maps/ThirdPersonMap.ThirdPersonMap"))))))))

(fn ConstructionScript
  (|CallParentFunction))