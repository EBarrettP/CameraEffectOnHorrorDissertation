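; A scripted scare prop: a vending machine that topples over when the phone is picked up.
; On BeginPlay it finds the BP_Phone actor in the level and binds its Fall event to the phone's pick-up event.
; Fall plays an attenuated impact sound at the furniture mesh, starting partway into the clip, while a timeline drives the root component's roll to tip the machine.
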(event Custom|Fall
  (bind _defaultsceneroot (Variables|Default|GetDefaultSceneRoot))
  (bind _relativerotation (Variables|/Script/Engine.SceneComponent|GetRelativeRotation _defaultsceneroot))
  (Audio|PlaySoundatLocation "/Game/EMsAssets/Audio/SoundSnap/SpookySounds/VendingMachine/220198-Impacts-SIMPLE-242.220198-Impacts-SIMPLE-242" (Transformation|GetWorldLocation (Variables|Default|GetFurnitureMesh)) "0, 0, 0" 1.0 1.0 4.0 "/Game/EMsAssets/Audio/BasicSoundAttenuation.BasicSoundAttenuation" 0 0 0)
  (bind _newtrack_0 (Timeline|Timeline_0 Play)
    (:Update
      (Transformation|SetRelativeRotation _defaultsceneroot (Math|Rotator|MakeRotator _newtrack_0 (.pitch _relativerotation) (.yaw _relativerotation)) false false))))

(event EventBeginPlay
  (|CallParentFunction)
  (bind _returnvalue (Actor|GetActorOfClass "/Game/EMsAssets/Objects/BP_Phone.BP_Phone_C"))
  (Variables|Default|SetPhone _returnvalue)
  (EventDispatchers|BindEventtoPickUpPhone (Variables|Default|GetPhone) (delegate Custom|Fall)))

(event Collision|EventActorBeginOverlap
  (params (OtherActor :type Actor%20Object%20Reference))
  (|CallParentFunction OtherActor) ; This node is disabled and will not be called.\nDrag off pins to build functionality.
)

(event EventTick
  (params (DeltaSeconds :type Float%20%28single-precision%29))
  (|CallParentFunction DeltaSeconds) ; This node is disabled and will not be called.\nDrag off pins to build functionality.
)

(fn ConstructionScript
  (|CallParentFunction))